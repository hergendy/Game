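; Tower actor that targets nearby ThirdPersonCharacter actors and fires arrows at them.
; Without a target, Tick scans all characters and keeps the last one within a fixed horizontal radius.
; With a target, a Delay on Tick paces TowerArrow spawns, passing each the target, until it leaves range.
; Spawn rotation takes raw position differences as rotator angles rather than computing a look-at rotation.
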(event `self.ReceiveTick`
  (params (DeltaSeconds :type "Float (single-precision)"))
  (bind _returnvalue (`self.K2_GetActorLocation`))
  (bind _currenttarget (`self.CurrentTarget`))
  (bind _returnvalue_2 (`SceneComponent.K2_GetComponentLocation` (`self.ArrowSpawn`)))
  (if (`self.HaveTarget`)
    (`KismetSystemLibrary.Delay` 1.0)
    (if (< (`KismetMathLibrary.Sqrt` (+ (`KismetMathLibrary.Square` (.x (- _returnvalue (`self.K2_GetActorLocation` _currenttarget)))) (`KismetMathLibrary.Square` (.y (- _returnvalue (`self.K2_GetActorLocation` _currenttarget)))))) 1000.0)
      (bind _returnvalue_3 (`|SpawnActorFromClass` "/Game/Blueprints/TowerArrow.TowerArrow_C" (`KismetMathLibrary.MakeTransform` _returnvalue_2 (`KismetMathLibrary.MakeRotator` (- (.x _returnvalue_2) (.x (`SceneComponent.K2_GetComponentLocation` (`Character.Mesh` _currenttarget)))) (- (.y _returnvalue_2) (.y (`SceneComponent.K2_GetComponentLocation` (`Character.Mesh` _currenttarget)))) (- (.z _returnvalue_2) (.z (`SceneComponent.K2_GetComponentLocation` (`Character.Mesh` _currenttarget)))))) "Undefined" "OverrideRootScale" null null))
      (`/Game/Blueprints/TowerArrow.ArrowSpawn` _returnvalue_3 _currenttarget)
      (else
        (set `self.HaveTarget` false)))
    (else
      (bind _outactors (`GameplayStatics.GetAllActorsOfClass` "/Game/ThirdPersonBP/Blueprints/ThirdPersonCharacter.ThirdPersonCharacter_C"))
      (for _array_element _outactors
        (if (< (`KismetMathLibrary.Sqrt` (+ (`KismetMathLibrary.Square` (.x (- (`self.K2_GetActorLocation` _array_element) _returnvalue))) (`KismetMathLibrary.Square` (.y (- (`self.K2_GetActorLocation` _array_element) _returnvalue))))) 1000.0)
          (set `self.CurrentTarget` _array_element)
          (set `self.HaveTarget` true))))))

(fn `UserConstructionScript`)