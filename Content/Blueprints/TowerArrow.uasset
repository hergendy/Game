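; TowerArrow is an arrow projectile, named for tower use, that launches as a physics-driven shaft relative to a target body.
; Its ArrowSpawn event replaces the Shaft's linear velocity with half the offset from the target's mesh to the Shaft.
; As written, that vector points away from the target, and its speed scales with distance.
; A manual distance calculation is left unconnected.
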(event `ArrowSpawn`
  (params (Target_Body :type "/Game/ThirdPersonBP/Blueprints/ThirdPersonCharacter Object Reference"))
  (bind _shaft (`self.Shaft`))
  (`PrimitiveComponent.SetAllPhysicsLinearVelocity` _shaft (/ (- (`SceneComponent.K2_GetComponentLocation` _shaft) (`SceneComponent.K2_GetComponentLocation` (`Character.Mesh` Target_Body))) 2.0) false))

(fn `UserConstructionScript`)